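; Game mode for a lane-based runner that, at BeginPlay, creates the HUD and adds it to the player screen.
; An unconnected, never-executed graph holds coin spawning: a weighted roll places a coin above a random lane of the last spawned tile.
; Further coins continue in a line along negative Y while a decreasing chance succeeds, each attached to that tile, then the chance resets.
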(event `self.ReceiveBeginPlay`
  (bind _returnvalue (`|CreateWidget` "/Game/Core/BP_HUD.BP_HUD_C"))
  (`UserWidget.AddToPlayerScreen` _returnvalue 0))

(fn `UserConstructionScript`)